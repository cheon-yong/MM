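; BP_Mercenary_Puppet is a modular mercenary character assembled from separate body, hand, feet, hair and mask meshes.
; The construction script sets the main Mesh as leader pose for all parts, keeping their animations in sync.
; The event graph holds timelines for blinking and eyebrow-raise morph targets that replay after random delays.
; Nothing starts either timeline in this graph, so that facial animation never runs.
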(fn `UserConstructionScript`
  ;[1 1 1] Sync Animations
  (`SkinnedMeshComponent.SetLeaderPoseComponent` (`self.UpperBody`) (`self.Mesh`) false false)
  (`SkinnedMeshComponent.SetLeaderPoseComponent` (`self.Feet`) (`self.Mesh`) false false)
  (`SkinnedMeshComponent.SetLeaderPoseComponent` (`self.Hand_L`) (`self.Mesh`) false false)
  (`SkinnedMeshComponent.SetLeaderPoseComponent` (`self.BottomBody`) (`self.Mesh`) false false)
  (`SkinnedMeshComponent.SetLeaderPoseComponent` (`self.Hand_R`) (`self.Mesh`) false false)
  (`SkinnedMeshComponent.SetLeaderPoseComponent` (`self.Long Hair`) (`self.Mesh`) false false)
  (`SkinnedMeshComponent.SetLeaderPoseComponent` (`self.Mask`) (`self.Mesh`) false false))