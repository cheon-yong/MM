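; BP_Langa is a character Blueprint with camera zoom and a hit-flicker effect.
; Zoom inputs step the CameraBoom arm length within a clamped range, and the T key executes the GameplayCue.Hit.Flicker cue on itself.
; SetRed, with no caller in this graph, stores mesh materials in OriginMaterials, applies FlickerMat dynamic instances, and restores the originals after a short Delay wired inside the swap loop.
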(event `InputAction|Zoom Out`
  (params (Key :type "Key Structure"))
  (bind _cameraboom (`self.CameraBoom`))
  (:`Pressed`
    (set `SpringArmComponent.TargetArmLength` (`KismetMathLibrary.FClamp` (+ (`SpringArmComponent.TargetArmLength` _cameraboom) -50.0) 200.0 3000.0) _cameraboom)))

(event `InputAction|Zoom In`
  (params (Key :type "Key Structure"))
  (bind _cameraboom (`self.CameraBoom`))
  (:`Pressed`
    (set `SpringArmComponent.TargetArmLength` (`KismetMathLibrary.FClamp` (+ (`SpringArmComponent.TargetArmLength` _cameraboom) 50.0) 200.0 3000.0) _cameraboom)))

(event `Key|T`
  (params (Key :type "Key Structure"))
  (:`Pressed`
    (`GameplayCueFunctionLibrary.ExecuteGameplayCueOnActor` self (struct :`TagName` "GameplayCue.Hit.Flicker") (`AbilitySystemBlueprintLibrary.MakeGameplayCueParameters` 0.0))))

(event `Set Red`
  (for (_array_element _array_index) (`MeshComponent.GetMaterials` (`self.Mesh`))
    (`KismetArrayLibrary.Array_Add` (`self.OriginMaterials`) _array_element)
    (bind _returnvalue (`KismetMaterialLibrary.CreateDynamicMaterialInstance` (`self.FlickerMat`)))
    (`PrimitiveComponent.SetMaterial` (`self.Mesh`) _array_index _returnvalue)
    (`KismetSystemLibrary.Delay` 0.2)
    (for (_array_element_2 _array_index_2) (`self.OriginMaterials`)
      (`PrimitiveComponent.SetMaterial` (`self.Mesh`) _array_index_2 _array_element_2))))

(fn `UserConstructionScript`)