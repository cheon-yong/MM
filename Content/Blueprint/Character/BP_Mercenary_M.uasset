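; Modular male mercenary character Blueprint with a zoomable camera boom.
; The construction script makes the body-part, hair and mask meshes follow the main Mesh's pose through Leader Pose Component.
; Zoom inputs step the boom's arm length within clamped limits, with Zoom Out shortening it and Zoom In lengthening it.
; Randomly delayed blink and eyebrow morph-target timelines are present but unconnected, so they never run.
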(event `InputAction|Zoom Out`
  (params (Key :type "Key Structure"))
  (bind _cameraboom (`self.CameraBoom`))
  (:`Pressed`
    (set `SpringArmComponent.TargetArmLength` (`KismetMathLibrary.FClamp` (+ (`SpringArmComponent.TargetArmLength` _cameraboom) -50.0) 200.0 3000.0) _cameraboom)))

(event `InputAction|Zoom In`
  (params (Key :type "Key Structure"))
  (bind _cameraboom (`self.CameraBoom`))
  (:`Pressed`
    (set `SpringArmComponent.TargetArmLength` (`KismetMathLibrary.FClamp` (+ (`SpringArmComponent.TargetArmLength` _cameraboom) 50.0) 200.0 3000.0) _cameraboom)))

(fn `UserConstructionScript`
  ;[1 1 1] Sync Animations
  (`SkinnedMeshComponent.SetLeaderPoseComponent` (`self.UpperBody`) (`self.Mesh`) false false)
  (`SkinnedMeshComponent.SetLeaderPoseComponent` (`self.Feet`) (`self.Mesh`) false false)
  (`SkinnedMeshComponent.SetLeaderPoseComponent` (`self.Hand_L`) (`self.Mesh`) false false)
  (`SkinnedMeshComponent.SetLeaderPoseComponent` (`self.BottomBody`) (`self.Mesh`) false false)
  (`SkinnedMeshComponent.SetLeaderPoseComponent` (`self.Hand_R`) (`self.Mesh`) false false)
  (`SkinnedMeshComponent.SetLeaderPoseComponent` (`self.Long Hair`) (`self.Mesh`) false false)
  (`SkinnedMeshComponent.SetLeaderPoseComponent` (`self.Mask`) (`self.Mesh`) false false))