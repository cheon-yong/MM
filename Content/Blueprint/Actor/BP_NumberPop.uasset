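; BP_NumberPop is a floating number popup actor that displays text through an MMNumberPopText widget component.
; BeginPlay caches the widget, and PlayTextAnimation records the current location as the origin before playing a Timeline.
; The Timeline offsets the actor from that origin and drives the alpha of the text and its shadow, both tinted white.
; When it finishes, the actor hands itself back to MMNumberPopSubsystem through ReturnActor.
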(event `self.ReceiveBeginPlay`
  (set `self.OriginLoc` (`self.K2_GetActorLocation`))
  (bind _asmmnumber_pop_text (cast `MMNumberPopText` (`WidgetComponent.GetWidget` (`self.NumberPop`))))
  (set `self.Text` _asmmnumber_pop_text))

(event `self.PlayTextAnimation`
  (set `self.OriginLoc` (`self.K2_GetActorLocation`))
  (bind (_direction _positionoffset _alpha) (`Timeline|Timeline`)
    (:`Update`
      (`self.K2_SetActorLocation` (+ _positionoffset (`self.OriginLoc`)))
      (bind _linearcolor (make `LinearColor` 1.0 1.0 1.0 _alpha))
      (set `TextBlock.ColorAndOpacity` (make `SlateColor` _linearcolor) (`MMNumberPopText.NumberText` (`self.Text`)))
      (`TextBlock.SetShadowColorAndOpacity` (`MMNumberPopText.NumberText` (`self.Text`)) _linearcolor))
    (:`Finished`
      (`MMNumberPopSubsystem.ReturnActor` (subsystem `MMNumberPopSubsystem`) self))))

(fn `UserConstructionScript`)