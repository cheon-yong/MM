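; Component that assembles segmented anime characters and gives each mesh segment an outline.
; Setup functions assign meshes to components and call CreateOutline; SetupCharacter also attaches hair to the head's socket.
; CreateOutline layers a duplicate skeletal mesh following the source's pose, reusing any valid OutlineMeshes entry.
; DT_AnimeMaterials rows, keyed by material slot name, set outline color and thickness or blank the slot, with M_Outline as fallback.
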(fn `Create Outline`
  (params (Owner :type "SkeletalMeshComponent Object Reference"))
  (returns (OutlineComp :type "SkeletalMeshComponent Object Reference"))
  (locals (LocalNewSkel :type "SkeletalMeshComponent Object Reference") (LocalDynaMat :type "MaterialInstanceDynamic Object Reference"))
  (bind _localnewskel (`local.LocalNewSkel`))
  (bind _localnewskel_2 (`local.LocalNewSkel`))
  (bind _localdynamat (`local.LocalDynaMat`))
  (bind (_value _returnvalue) (`BlueprintMapLibrary.Map_Find` (`self.OutlineMeshes`) Owner))
  (if _returnvalue
    (`/Engine/EditorBlueprintResources/StandardMacros.IsValid` _value
      (:`Is Valid`
        (set `local.LocalNewSkel` _value))
      (:`Is Not Valid`
        (bind _returnvalue_2 (`|AddComponentByClass` :`self` (`self.GetOwner`) :`Class` "/Script/Engine.SkeletalMeshComponent" :!label _label))
        (set `local.LocalNewSkel` _returnvalue_2)))
    (else
      (goto _label)))
  (`SkinnedMeshComponent.SetSkinnedAssetAndUpdate` _localnewskel (`SkeletalMeshComponent.GetSkeletalMeshAsset` Owner) true)
  (`SkinnedMeshComponent.SetLeaderPoseComponent` _localnewskel Owner true false)
  (`SceneComponent.K2_AttachToComponent` _localnewskel (`local.Owner`) "None" "SnapToTarget" "SnapToTarget" "SnapToTarget" true)
  (for (_ _array_index) (`MeshComponent.GetMaterials` Owner)
    ;[1 1 1] Modify Outline
    (bind _returnvalue_3 (`|GetDataTableRow` "/Game/AnimeCharacters/Blueprints/Misc/DT_AnimeMaterials.DT_AnimeMaterials" (`|GetArrayItem` (`MeshComponent.GetMaterialSlotNames` Owner) _array_index))
      (:`then`
        (bind _returnvalue_4 (`KismetMaterialLibrary.CreateDynamicMaterialInstance` "/Game/AnimeCharacters/Materials/m_Outline.m_Outline"))
        (bind _output_get (set `local.LocalDynaMat` _returnvalue_4))
        (`PrimitiveComponent.SetMaterial` _localnewskel_2 _array_index (select `bool` (`.NoOutline_1_19E658B84C90865316C1CDAA6D536837` (break `/Game/AnimeCharacters/Blueprints/Misc/st_AnimeMaterialData` _returnvalue_3)) :`false` _output_get :`true` "/Game/AnimeCharacters/Materials/m_blank.m_blank" :!type "MaterialInterface Object Reference"))
        (bind (_nooutline _outlinecolor _outlinethinkness) (break `/Game/AnimeCharacters/Blueprints/Misc/st_AnimeMaterialData` _returnvalue_3))
        (if (not _nooutline)
          (`MaterialInstanceDynamic.SetVectorParameterValue` _localdynamat "Color" _outlinecolor)
          (`MaterialInstanceDynamic.SetScalarParameterValue` _localdynamat "Thickness" _outlinethinkness)))
      (:`RowNotFound`
        (`PrimitiveComponent.SetMaterial` _localnewskel_2 _array_index "/Game/AnimeCharacters/Materials/m_Outline.m_Outline"))))
  (return (`local.LocalNewSkel`)))

(fn `SetupCharacter`
  (params (`Head Comp` :type "SkeletalMeshComponent Object Reference") (`Hair Comp` :type "SkeletalMeshComponent Object Reference") (Components :type "Array of SkeletalMeshComponent Object Reference (by ref)") (Meshes :type "Array of SkeletalMesh Object Reference (by ref)"))
  (`SceneComponent.K2_AttachToComponent` `Hair Comp` `Head Comp` "HeadAttachment" "KeepRelative" "KeepRelative" "KeepRelative" true)
  (for (_array_element _array_index) Meshes
    (bind _output (`|GetArrayItem` Components _array_index))
    (`SkinnedMeshComponent.SetSkinnedAssetAndUpdate` _output _array_element true)
    (`self.Create Outline` _output)))

(fn `SetupMeshSegments`
  (params (Components :type "Array of SkeletalMeshComponent Object Reference") (Meshes :type "Array of SkeletalMesh Object Reference"))
  (for (_array_element _array_index) Meshes
    (bind _output (`|GetArrayItem` Components _array_index))
    (`SkinnedMeshComponent.SetSkinnedAssetAndUpdate` _output _array_element true)
    (`self.Create Outline` _output)))